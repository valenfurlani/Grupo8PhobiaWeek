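; Base portal actor that teleports the game to another level.
; Any overlap with its box collider opens the referenced Level, with no check on what entered.
; Each tick the root turns to face the player character.
; The construction script points a cube scene capture at TextureForTheOtherLevel, apparently for the other level's use, and applies the configured material to the portal.
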(event OnComponentBeginOverlap(BoxCollider)
  (params (OverlappedComponent :type Primitive%20Component%20Object%20Reference) (OtherActor :type Actor%20Object%20Reference) (OtherComp :type Primitive%20Component%20Object%20Reference) (OtherBodyIndex :type Integer) (bFromSweep :type Boolean) (SweepResult :type Hit%20Result%20Structure%20%28by%20ref%29))
  (Game|OpenLevel(byObjectReference) (Variables|Default|GetLevel)))

(event EventTick
  (params (DeltaSeconds :type Float%20%28single-precision%29))
  (Transformation|SetWorldRotation (Variables|Default|GetDefaultSceneRoot) (Math|Rotator|FindLookatRotation (Transformation|GetWorldLocation (Variables|Default|GetDefaultSceneRoot)) (Transformation|GetActorLocation (Game|GetPlayerCharacter 0))) false false))

(fn ConstructionScript
  (Variables|/Script/Engine.SceneCaptureComponentCube|SetTextureTarget (Variables|Default|GetSceneCaptureComponentCube) (Variables|Default|GetTexture%20for%20the%20other%20level))
  (Rendering|Material|SetMaterial (Variables|Default|GetPortal) 0 (Variables|Default|GetMaterial)))